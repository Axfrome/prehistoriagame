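; Game mode Blueprint that respawns the first player's survival character whenever it is destroyed.
; On BeginPlay it binds to the character's OnDestroyed event.
; After destruction it waits briefly, spawns a new BP_SurvivalCharacter at SpawnTransform, possesses it with player controller 0, then calls Respawn to rebind the event and keep the cycle going.
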(event Custom|OnDestroyed_
  (params (DestroyedActor :type Actor%20Object%20Reference))
  (Utilities|FlowControl|Delay 2.0)
  (bind _returnvalue (Game|SpawnActorfromClass "/Game/Prog/Systemes/Personnage/Principal/BP_SurvivalCharacter.BP_SurvivalCharacter_C" (Variables|Default|GetSpawnTransform) "AlwaysSpawn" 0 0))
  (Pawn|Possess (Game|GetPlayerController 0) _returnvalue)
  (CallFunction|Respawn))

(event Custom|Respawn
  (bind _asbp_survival_character (Utilities|Casting|CastToBP_SurvivalCharacter (Game|GetPlayerCharacter 0)))
  (Game|BindEventtoOnDestroyed _asbp_survival_character (delegate Custom|OnDestroyed_)))

(event EventBeginPlay
  (bind _asbp_survival_character (Utilities|Casting|CastToBP_SurvivalCharacter (Game|GetPlayerCharacter 0)))
  (Game|BindEventtoOnDestroyed _asbp_survival_character (delegate Custom|OnDestroyed_)))

(fn ConstructionScript)