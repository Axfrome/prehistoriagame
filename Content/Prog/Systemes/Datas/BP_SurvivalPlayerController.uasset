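; Survival player controller that opens the game's front-end widgets (menus, settings, loading screens, credits and similar) in English, French, German, Italian and Spanish.
; Each screen and language pair has its own event that creates and caches the widget and adds it to the viewport.
; Several events cache into mismatched variables, notably English widgets into French slots.
; ApplySettings applies quality presets, resolution, window mode and VSync through console commands.
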(event Custom|HUD%20-%20Graph%20-%20ENG
  ;[1 1 1] Widgets ENG
  ;;[1 1 1] Create Graphic ENG
  (Utilities|IsValid (Variables|Default|GetGraphic_ENG)
    (:Is%20Valid
      _)
    (:Is%20Not%20Valid
      (bind _returnvalue (UserInterface|CreateWidget "/Game/Prog/Systemes/Menu/Widgets/ENG/Graphic_ENG.Graphic_ENG_C"))
      (Variables|Default|SetGraphic_FR _returnvalue)))
  (UserInterface|Viewport|AddtoViewport _returnvalue 0))

(event Custom|HUD%20-%20Setting%20-%20FR
  (Utilities|IsValid (Variables|Default|GetSetting_FR)
    (:Is%20Valid
      _)
    (:Is%20Not%20Valid
      (bind _returnvalue (UserInterface|CreateWidget "/Game/Prog/Systemes/Menu/Widgets/FR/Setting_FR.Setting_FR_C"))
      (Variables|Default|SetSetting_FR _returnvalue)))
  (UserInterface|Viewport|AddtoViewport _returnvalue 0))

(event Custom|HUD-%20Menu%20-%20FR
  (Utilities|IsValid (Variables|Default|GetMenu_FR)
    (:Is%20Valid
      _)
    (:Is%20Not%20Valid
      (bind _returnvalue (UserInterface|CreateWidget "/Game/Prog/Systemes/Menu/Widgets/FR/MenuMain_FR.MenuMain_FR_C"))
      (Variables|Default|SetMenu_FR _returnvalue)))
  (UserInterface|Viewport|AddtoViewport _returnvalue 0))

(event Custom|HUD%20-%20Control%20-%20FR
  (Utilities|IsValid (Variables|Default|GetControl_FR)
    (:Is%20Valid
      _)
    (:Is%20Not%20Valid
      (bind _returnvalue (UserInterface|CreateWidget "/Game/Prog/Systemes/Menu/Widgets/FR/Control_FR.Control_FR_C"))
      (Variables|Default|SetControl_FR _returnvalue)))
  (UserInterface|Viewport|AddtoViewport _returnvalue 0))

(event Custom|HUD%20-%20Audio%20-%20ENG
  ;[1 1 1] Widgets ENG
  ;;[1 1 1] Create Audio ENG
  (Utilities|IsValid (Variables|Default|GetAudio_ENG)
    (:Is%20Valid
      _)
    (:Is%20Not%20Valid
      (bind _returnvalue (UserInterface|CreateWidget "/Game/Prog/Systemes/Menu/Widgets/ENG/Audio_ENG.Audio_ENG_C"))
      (Variables|Default|SetAudio_FR _returnvalue)))
  (UserInterface|Viewport|AddtoViewport _returnvalue 0))

(event Custom|HUD%20-%20Setting%20-%20ITA
  (Utilities|IsValid (Variables|Default|GetSetting_ITA)
    (:Is%20Valid
      _)
    (:Is%20Not%20Valid
      (bind _returnvalue (UserInterface|CreateWidget "/Game/Prog/Systemes/Menu/Widgets/ITA/Setting_ITA.Setting_ITA_C"))
      (Variables|Default|SetSetting_ITA _returnvalue)))
  (UserInterface|Viewport|AddtoViewport _returnvalue 0))

(event Custom|HUD%20-%20Loading%20-%20ITA
  (Utilities|IsValid (Variables|Default|GetLoading_ITA)
    (:Is%20Valid
      _)
    (:Is%20Not%20Valid
      (bind _returnvalue (UserInterface|CreateWidget "/Game/Prog/Systemes/Menu/Widgets/ITA/LoadingScreen_ITA.LoadingScreen_ITA_C"))
      (Variables|Default|SetLoading_ITA _returnvalue)))
  (UserInterface|Viewport|AddtoViewport _returnvalue 0))

(event Custom|HUD%20-%20Credits%20-%20FR
  (Utilities|IsValid (Variables|Default|GetCredit_FR)
    (:Is%20Valid
      _)
    (:Is%20Not%20Valid
      (bind _returnvalue (UserInterface|CreateWidget "/Game/Prog/Systemes/Menu/Widgets/FR/Credit_FR.Credit_FR_C"))
      (Variables|Default|SetCredit_FR _returnvalue)))
  (UserInterface|Viewport|AddtoViewport _returnvalue 0))

(event Custom|HUD%20-%20Selection%20-%20FR
  (Utilities|IsValid (Variables|Default|GetSelection_FR)
    (:Is%20Valid
      _)
    (:Is%20Not%20Valid
      (bind _returnvalue (UserInterface|CreateWidget "/Game/Prog/Systemes/Menu/Widgets/FR/Selection_FR.Selection_FR_C"))
      (Variables|Default|SetSelection_FR _returnvalue)))
  (UserInterface|Viewport|AddtoViewport _returnvalue 0))

(event Custom|Coop_ENG
  (Utilities|IsValid (Variables|Default|GetLanguage_FR)
    (:Is%20Valid
      _)
    (:Is%20Not%20Valid
      (bind _returnvalue (UserInterface|CreateWidget "/Game/Prog/Systemes/Menu/Widgets/ENG/Coop_ENG.Coop_ENG_C"))
      (Variables|Default|SetCoop _returnvalue)))
  (UserInterface|Viewport|AddtoViewport _returnvalue 0))

(event Custom|HUD%20-%20Audio%20-%20FR
  (Utilities|IsValid (Variables|Default|GetAudio_FR)
    (:Is%20Valid
      _)
    (:Is%20Not%20Valid
      (bind _returnvalue (UserInterface|CreateWidget "/Game/Prog/Systemes/Menu/Widgets/FR/Audio_FR.Audio_FR_C"))
      (Variables|Default|SetAudio_FR _returnvalue)))
  (UserInterface|Viewport|AddtoViewport _returnvalue 0))

(event Custom|HUD%20-%20Graph%20-%20FR
  (Utilities|IsValid (Variables|Default|GetGraphic_FR)
    (:Is%20Valid
      _)
    (:Is%20Not%20Valid
      (bind _returnvalue (UserInterface|CreateWidget "/Game/Prog/Systemes/Menu/Widgets/FR/Graphic_FR.Graphic_FR_C"))
      (Variables|Default|SetGraphic_FR _returnvalue)))
  (UserInterface|Viewport|AddtoViewport _returnvalue 0))

(event Custom|HUD-%20Menu%20-%20ENG
  ;[1 1 1] Widgets ENG
  ;;[1 1 1] Create Menu ENG
  (Utilities|IsValid (Variables|Default|GetMenu_ENG)
    (:Is%20Valid
      _)
    (:Is%20Not%20Valid
      (bind _returnvalue (UserInterface|CreateWidget "/Game/Prog/Systemes/Menu/Widgets/ENG/MenuMain_ENG.MenuMain_ENG_C"))
      (Variables|Default|SetMenu_FR _returnvalue)))
  (UserInterface|Viewport|AddtoViewport _returnvalue 0)
  (Variables|Default|SetbShowMouseCursor true))

(event Custom|HUD%20-%20Setting%20-%20ESP
  (Utilities|IsValid (Variables|Default|GetSetting_ESP)
    (:Is%20Valid
      _)
    (:Is%20Not%20Valid
      (bind _returnvalue (UserInterface|CreateWidget "/Game/Prog/Systemes/Menu/Widgets/ESP/Setting_ESP.Setting_ESP_C"))
      (Variables|Default|SetSetting_ESP _returnvalue)))
  (UserInterface|Viewport|AddtoViewport _returnvalue 0))

(event Custom|HUD%20-%20Loading%20-%20ESP
  (Utilities|IsValid (Variables|Default|GetLoading_ESP)
    (:Is%20Valid
      _)
    (:Is%20Not%20Valid
      (bind _returnvalue (UserInterface|CreateWidget "/Game/Prog/Systemes/Menu/Widgets/ESP/LoadingScreen_esp.LoadingScreen_ESP_C"))
      (Variables|Default|SetLoading_ESP _returnvalue)))
  (UserInterface|Viewport|AddtoViewport _returnvalue 0))

(event Custom|HUD-%20Menu%20-%20ESP
  (Utilities|IsValid (Variables|Default|GetMenu_ESP)
    (:Is%20Valid
      _)
    (:Is%20Not%20Valid
      (bind _returnvalue (UserInterface|CreateWidget "/Game/Prog/Systemes/Menu/Widgets/ESP/MenuMain_ESP.MenuMain_ESP_C"))
      (Variables|Default|SetMenu_ESP _returnvalue)))
  (UserInterface|Viewport|AddtoViewport _returnvalue 0))

(event Custom|HUD%20-%20Control%20-%20ESP
  (Utilities|IsValid (Variables|Default|GetControl_ESP)
    (:Is%20Valid
      _)
    (:Is%20Not%20Valid
      (bind _returnvalue (UserInterface|CreateWidget "/Game/Prog/Systemes/Menu/Widgets/ESP/Control_ESP.Control_ESP_C"))
      (Variables|Default|SetControl_ESP _returnvalue)))
  (UserInterface|Viewport|AddtoViewport _returnvalue 0))

(event Custom|HUD%20-%20Audio%20-%20ESP
  (Utilities|IsValid (Variables|Default|GetAudio_ESP)
    (:Is%20Valid
      _)
    (:Is%20Not%20Valid
      (bind _returnvalue (UserInterface|CreateWidget "/Game/Prog/Systemes/Menu/Widgets/ESP/Audio_ESP.Audio_ESP_C"))
      (Variables|Default|SetAudio_ESP _returnvalue)))
  (UserInterface|Viewport|AddtoViewport _returnvalue 0))

(event Custom|HUD%20-%20Graph%20-%20ESP
  (Utilities|IsValid (Variables|Default|GetGraphic_ESP)
    (:Is%20Valid
      _)
    (:Is%20Not%20Valid
      (bind _returnvalue (UserInterface|CreateWidget "/Game/Prog/Systemes/Menu/Widgets/ESP/Graphic_ESP.Graphic_ESP_C"))
      (Variables|Default|SetGraphic_ESP _returnvalue)))
  (UserInterface|Viewport|AddtoViewport _returnvalue 0))

(event Custom|HUD%20-%20Credits%20-%20ESP
  (Utilities|IsValid (Variables|Default|GetCredit_ESP)
    (:Is%20Valid
      _)
    (:Is%20Not%20Valid
      (bind _returnvalue (UserInterface|CreateWidget "/Game/Prog/Systemes/Menu/Widgets/ESP/Credit_ESP.Credit_ESP_C"))
      (Variables|Default|SetCredit_ESP _returnvalue)))
  (UserInterface|Viewport|AddtoViewport _returnvalue 0))

(event Custom|HUD%20-%20Selection%20-%20ESP
  (Utilities|IsValid (Variables|Default|GetSelection_ESP)
    (:Is%20Valid
      _)
    (:Is%20Not%20Valid
      (bind _returnvalue (UserInterface|CreateWidget "/Game/Prog/Systemes/Menu/Widgets/ESP/Selection_ESP.Selection_ESP_C"))
      (Variables|Default|SetSelection_ESP _returnvalue)))
  (UserInterface|Viewport|AddtoViewport _returnvalue 0))

(event Custom|HUD%20-%20Language%20-%20ESP
  (Utilities|IsValid (Variables|Default|GetLanguage_ESP)
    (:Is%20Valid
      _)
    (:Is%20Not%20Valid
      (bind _returnvalue (UserInterface|CreateWidget "/Game/Prog/Systemes/Menu/Widgets/ESP/Languages_esp.Languages_ESP_C"))
      (Variables|Default|SetLanguage_ESP _returnvalue)))
  (UserInterface|Viewport|AddtoViewport _returnvalue 0))

(event Custom|HUD-%20Menu%20-%20ITA
  (Utilities|IsValid (Variables|Default|GetMenu_ITA)
    (:Is%20Valid
      _)
    (:Is%20Not%20Valid
      (bind _returnvalue (UserInterface|CreateWidget "/Game/Prog/Systemes/Menu/Widgets/ITA/MenuMain_ITA.MenuMain_ITA_C"))
      (Variables|Default|SetMenu_ITA _returnvalue)))
  (UserInterface|Viewport|AddtoViewport _returnvalue 0))

(event Custom|HUD%20-%20Credits%20-%20ENG
  ;[1 1 1] Widgets ENG
  ;;[1 1 1] Create credits ENG
  (Utilities|IsValid (Variables|Default|GetCredit_ENG)
    (:Is%20Valid
      _)
    (:Is%20Not%20Valid
      (bind _returnvalue (UserInterface|CreateWidget "/Game/Prog/Systemes/Menu/Widgets/ENG/Credit_ENG.Credit_ENG_C"))
      (Variables|Default|SetCredit_FR _returnvalue)))
  (UserInterface|Viewport|AddtoViewport _returnvalue 0))

(event Custom|HUD%20-%20Control%20-%20ITA
  (Utilities|IsValid (Variables|Default|GetControl_ITA)
    (:Is%20Valid
      _)
    (:Is%20Not%20Valid
      (bind _returnvalue (UserInterface|CreateWidget "/Game/Prog/Systemes/Menu/Widgets/ITA/Control_ITA.Control_ITA_C"))
      (Variables|Default|SetAudio_ITA _returnvalue)))
  (UserInterface|Viewport|AddtoViewport _returnvalue 0))

(event Custom|HUD%20-%20Audio%20-%20ITA
  (Utilities|IsValid (Variables|Default|GetAudio_ITA)
    (:Is%20Valid
      _)
    (:Is%20Not%20Valid
      (bind _returnvalue (UserInterface|CreateWidget "/Game/Prog/Systemes/Menu/Widgets/ITA/Audio_ITA.Audio_ITA_C"))
      (Variables|Default|SetAudio_ITA _returnvalue)))
  (UserInterface|Viewport|AddtoViewport _returnvalue 0))

(event Custom|HUD%20-%20Graph%20-%20ITA
  (Utilities|IsValid (Variables|Default|GetGraphic_ITA)
    (:Is%20Valid
      _)
    (:Is%20Not%20Valid
      (bind _returnvalue (UserInterface|CreateWidget "/Game/Prog/Systemes/Menu/Widgets/ITA/Graphic_ITA.Graphic_ITA_C"))
      (Variables|Default|SetGraphic_ITA _returnvalue)))
  (UserInterface|Viewport|AddtoViewport _returnvalue 0))

(event Custom|HUD%20-%20Credits%20-%20ITA
  (Utilities|IsValid (Variables|Default|GetCredit_ITA)
    (:Is%20Valid
      (UserInterface|Viewport|AddtoViewport (stale _returnvalue) 0))
    (:Is%20Not%20Valid
      (bind _returnvalue (UserInterface|CreateWidget "/Game/Prog/Systemes/Menu/Widgets/ITA/Credit_ITA.Credit_ITA_C"))
      (Variables|Default|SetCredit_ITA _returnvalue))))

(event Custom|HUD%20-%20Selection%20-%20ITA
  (Utilities|IsValid (Variables|Default|GetSelection_ITA)
    (:Is%20Valid
      _)
    (:Is%20Not%20Valid
      (bind _returnvalue (UserInterface|CreateWidget "/Game/Prog/Systemes/Menu/Widgets/ITA/Selection_ITA.Selection_ITA_C"))
      (Variables|Default|SetSelection_ITA _returnvalue)))
  (UserInterface|Viewport|AddtoViewport _returnvalue 0))

(event Custom|HUD%20-%20Language%20-%20ITA
  (Utilities|IsValid (Variables|Default|GetLanguage_ITA)
    (:Is%20Valid
      _)
    (:Is%20Not%20Valid
      (bind _returnvalue (UserInterface|CreateWidget "/Game/Prog/Systemes/Menu/Widgets/ITA/Languages_ITA.Languages_ITA_C"))
      (Variables|Default|SetLanguage_ITA _returnvalue)))
  (UserInterface|Viewport|AddtoViewport _returnvalue 0))

(event Custom|HUD%20-%20Language%20-%20FR
  (Utilities|IsValid (Variables|Default|GetLanguage_FR)
    (:Is%20Valid
      _)
    (:Is%20Not%20Valid
      (bind _returnvalue (UserInterface|CreateWidget "/Game/Prog/Systemes/Menu/Widgets/FR/Languages_FR.Languages_FR_C"))
      (Variables|Default|SetLanguage_FR _returnvalue)))
  (UserInterface|Viewport|AddtoViewport _returnvalue 0))

(event Custom|HUD%20Language%20-%20ENG
  ;[1 1 1] Widgets ENG
  ;;[1 1 1] Create Languages ENG
  (Utilities|IsValid (Variables|Default|GetLanguage_ENG)
    (:Is%20Valid
      _)
    (:Is%20Not%20Valid
      (bind _returnvalue (UserInterface|CreateWidget "/Game/Prog/Systemes/Menu/Widgets/ENG/Languages_ENG.Languages_ENG_C"))
      (Variables|Default|SetLanguage_ENG _returnvalue)))
  (UserInterface|Viewport|AddtoViewport _returnvalue 0))

(event Custom|HUD%20-%20Loading%20-%20ENG
  ;[1 1 1] Widgets ENG
  ;;[1 1 1] Create loading screen ENG
  (Utilities|IsValid (Variables|Default|GetLoading_ENG)
    (:Is%20Valid
      _)
    (:Is%20Not%20Valid
      (bind _returnvalue (UserInterface|CreateWidget "/Game/Prog/Systemes/Menu/Widgets/ENG/LoadingScreen_ENG.LoadingScreen_ENG_C"))
      (Variables|Default|SetLoading_FR _returnvalue)))
  (UserInterface|Viewport|AddtoViewport _returnvalue 0))

(event Custom|HUD%20-%20Setting%20-%20ENG
  ;[1 1 1] Widgets ENG
  ;;[1 1 1] Create Settings ENG
  (Utilities|IsValid (Variables|Default|GetSetting_ENG)
    (:Is%20Valid
      _)
    (:Is%20Not%20Valid
      (bind _returnvalue (UserInterface|CreateWidget "/Game/Prog/Systemes/Menu/Widgets/ENG/Setting_ENG.Setting_ENG_C"))
      (Variables|Default|SetSetting_ENG _returnvalue)))
  (UserInterface|Viewport|AddtoViewport _returnvalue 0))

(event Custom|HUD%20-%20Setting%20-%20GER
  (Utilities|IsValid (Variables|Default|GetSetting_GER)
    (:Is%20Valid
      _)
    (:Is%20Not%20Valid
      (bind _returnvalue (UserInterface|CreateWidget "/Game/Prog/Systemes/Menu/Widgets/GER/Setting_GER.Setting_GER_C"))
      (Variables|Default|SetSetting_GER _returnvalue)))
  (UserInterface|Viewport|AddtoViewport _returnvalue 0))

(event Custom|ApplySettings
  (params (Quality :type E_GraphismesMenu%20Enum :default "NewEnumerator0") (WindowMode :type Boolean) (VSync :type Boolean) (ResolutionQuality :type Integer) (Resolution :type String))
  ;[1 1 1] Setting Graphic
  (Utilities|FlowControl|Sequence
    (:then_0
      (switch Utilities|FlowControl|Switch|SwitchonE_GraphismesMenu Quality
        (:NewEnumerator0
          (Development|ExecuteConsoleCommand "sg.ViewDistanceQuality 0" 0)
          (Development|ExecuteConsoleCommand "sg.AntiAliasingQuality 0" 0)
          (Development|ExecuteConsoleCommand "sg.PostProcessQuality 0" 0)
          (Development|ExecuteConsoleCommand "sg.ShadowQuality 0" 0)
          (Development|ExecuteConsoleCommand "sg.TextureQuality 0" 0)
          (Development|ExecuteConsoleCommand "sg.TextureQuality 0" 0)
          (Development|ExecuteConsoleCommand "sg.EffectsQuality 0" 0)
          (Development|ExecuteConsoleCommand "sg.FoliageQuality 0" 0))
        (:NewEnumerator1
          (Development|ExecuteConsoleCommand "sg.ViewDistanceQuality 1" 0)
          (Development|ExecuteConsoleCommand "sg.AntiAliasingQuality 1" 0)
          (Development|ExecuteConsoleCommand "sg.PostProcessQuality 1" 0)
          (Development|ExecuteConsoleCommand "sg.ShadowQuality 1" 0)
          (Development|ExecuteConsoleCommand "sg.TextureQuality 1" 0)
          (Development|ExecuteConsoleCommand "sg.TextureQuality 1" 0)
          (Development|ExecuteConsoleCommand "sg.EffectsQuality 1" 0)
          (Development|ExecuteConsoleCommand "sg.FoliageQuality 1" 0))
        (:NewEnumerator2
          (Development|ExecuteConsoleCommand "sg.ViewDistanceQuality 2" 0)
          (Development|ExecuteConsoleCommand "sg.AntiAliasingQuality 2" 0)
          (Development|ExecuteConsoleCommand "sg.PostProcessQuality 2" 0)
          (Development|ExecuteConsoleCommand "sg.ShadowQuality 2" 0)
          (Development|ExecuteConsoleCommand "sg.TextureQuality 2" 0)
          (Development|ExecuteConsoleCommand "sg.TextureQuality 2" 0)
          (Development|ExecuteConsoleCommand "sg.EffectsQuality 2" 0)
          (Development|ExecuteConsoleCommand "sg.FoliageQuality 2" 0))
        (:NewEnumerator3
          (Development|ExecuteConsoleCommand "sg.ViewDistanceQuality 3" 0)
          (Development|ExecuteConsoleCommand "sg.AntiAliasingQuality 3" 0)
          (Development|ExecuteConsoleCommand "sg.PostProcessQuality 3" 0)
          (Development|ExecuteConsoleCommand "sg.ShadowQuality 3" 0)
          (Development|ExecuteConsoleCommand "sg.TextureQuality 3" 0)
          (Development|ExecuteConsoleCommand "sg.TextureQuality 3" 0)
          (Development|ExecuteConsoleCommand "sg.EffectsQuality 3" 0)
          (Development|ExecuteConsoleCommand "sg.FoliageQuality 3" 0))))
    (:then_1
      (if WindowMode
        (Development|ExecuteConsoleCommand (Utilities|String|Append "r.SetRes " Resolution "f") 0)
        (else
          (Development|ExecuteConsoleCommand (Utilities|String|Append "r.SetRes " Resolution "w") 0))))
    (:then_2
      (if VSync
        (Development|ExecuteConsoleCommand (Utilities|String|Append "r.VSYNC " "1") 0)
        (else
          (Development|ExecuteConsoleCommand (Utilities|String|Append "r.VSYNC " "0") 0))))
    (:then_3
      (Development|ExecuteConsoleCommand (Utilities|String|Append "sg.ResolutionQuality " (Utilities|String|ToString(Integer) ResolutionQuality)) 0))))

(event Custom|HUD%20-%20Loading%20-%20GER
  (Utilities|IsValid (Variables|Default|GetLoading_GER)
    (:Is%20Valid
      _)
    (:Is%20Not%20Valid
      (bind _returnvalue (UserInterface|CreateWidget "/Game/Prog/Systemes/Menu/Widgets/GER/LoadingScreen_GER.LoadingScreen_GER_C"))
      (Variables|Default|SetLoading_GER _returnvalue)))
  (UserInterface|Viewport|AddtoViewport _returnvalue 0))

(event Custom|HUD-%20Menu%20-%20GER
  (Utilities|IsValid (Variables|Default|GetMenu_GER)
    (:Is%20Valid
      _)
    (:Is%20Not%20Valid
      (bind _returnvalue (UserInterface|CreateWidget "/Game/Prog/Systemes/Menu/Widgets/GER/MenuMain_GER.MenuMain_GER_C"))
      (Variables|Default|SetMenu_GER _returnvalue)))
  (UserInterface|Viewport|AddtoViewport _returnvalue 0))

(event Custom|HUD%20-%20Control%20-%20GER
  (Utilities|IsValid (Variables|Default|GetControl_GER)
    (:Is%20Valid
      _)
    (:Is%20Not%20Valid
      (bind _returnvalue (UserInterface|CreateWidget "/Game/Prog/Systemes/Menu/Widgets/GER/Control_GER.Control_GER_C"))
      (Variables|Default|SetAudio_GER _returnvalue)))
  (UserInterface|Viewport|AddtoViewport _returnvalue 0))

(event Custom|HUD%20-%20Audio%20-%20GER
  (Utilities|IsValid (Variables|Default|GetAudio_GER)
    (:Is%20Valid
      _)
    (:Is%20Not%20Valid
      (bind _returnvalue (UserInterface|CreateWidget "/Game/Prog/Systemes/Menu/Widgets/GER/Audio_GER.Audio_GER_C"))
      (Variables|Default|SetAudio_GER _returnvalue)))
  (UserInterface|Viewport|AddtoViewport _returnvalue 0))

(event Custom|HUD%20-%20Graph%20-%20GER
  (Utilities|IsValid (Variables|Default|GetGraphic_GER)
    (:Is%20Valid
      _)
    (:Is%20Not%20Valid
      (bind _returnvalue (UserInterface|CreateWidget "/Game/Prog/Systemes/Menu/Widgets/GER/Graphic_GER.Graphic_GER_C"))
      (Variables|Default|SetGraphic_GER _returnvalue)))
  (UserInterface|Viewport|AddtoViewport _returnvalue 0))

(event Custom|HUD%20-%20Language%20-%20GER
  (Utilities|IsValid (Variables|Default|GetLanguage_GER)
    (:Is%20Valid
      _)
    (:Is%20Not%20Valid
      (bind _returnvalue (UserInterface|CreateWidget "/Game/Prog/Systemes/Menu/Widgets/GER/Languages_GER.Languages_GER_C"))
      (Variables|Default|SetLanguage_GER _returnvalue)))
  (UserInterface|Viewport|AddtoViewport _returnvalue 0))

(event Custom|HUD%20-%20Credits%20-%20GER
  (Utilities|IsValid (Variables|Default|GetCredit_GER)
    (:Is%20Valid
      _)
    (:Is%20Not%20Valid
      (bind _returnvalue (UserInterface|CreateWidget "/Game/Prog/Systemes/Menu/Widgets/GER/Credit_GER.Credit_GER_C"))
      (Variables|Default|SetCredit_GER _returnvalue)))
  (UserInterface|Viewport|AddtoViewport _returnvalue 0))

(event Custom|HUD%20-%20Selection%20-%20GER
  (Utilities|IsValid (Variables|Default|GetSelection_GER)
    (:Is%20Valid
      _)
    (:Is%20Not%20Valid
      (bind _returnvalue (UserInterface|CreateWidget "/Game/Prog/Systemes/Menu/Widgets/GER/Selection_GER.Selection_GER_C"))
      (Variables|Default|SetSelection_GER _returnvalue)))
  (UserInterface|Viewport|AddtoViewport _returnvalue 0))

(event Custom|HUD%20-%20Selection%20-%20ENG
  ;[1 1 1] Widgets ENG
  ;;[1 1 1] Create Selection ENG
  (Utilities|IsValid (Variables|Default|GetSelection_ENG)
    (:Is%20Valid
      _)
    (:Is%20Not%20Valid
      (bind _returnvalue (UserInterface|CreateWidget "/Game/Prog/Systemes/Menu/Widgets/ENG/Selection_ENG.Selection_ENG_C"))
      (Variables|Default|SetSelection_FR _returnvalue)))
  (UserInterface|Viewport|AddtoViewport _returnvalue 0))

(event Custom|HUD%20-%20Control%20-%20ENG
  ;[1 1 1] Widgets ENG
  ;;[1 1 1] Create controls ENG
  (Utilities|IsValid (Variables|Default|GetControl_ENG)
    (:Is%20Valid
      _)
    (:Is%20Not%20Valid
      (bind _returnvalue (UserInterface|CreateWidget "/Game/Prog/Systemes/Menu/Widgets/ENG/Control_ENG.Control_ENG_C"))
      (Variables|Default|SetControl_FR _returnvalue)))
  (UserInterface|Viewport|AddtoViewport _returnvalue 0))

(event Custom|HUD%20-%20Loading%20-%20FR
  (Utilities|IsValid (Variables|Default|GetLoading_FR)
    (:Is%20Valid
      _)
    (:Is%20Not%20Valid
      (bind _returnvalue (UserInterface|CreateWidget "/Game/Prog/Systemes/Menu/Widgets/FR/LoadingScreen_FR.LoadingScreen_FR_C"))
      (Variables|Default|SetLoading_FR _returnvalue)))
  (UserInterface|Viewport|AddtoViewport _returnvalue 0))

(fn ConstructionScript)