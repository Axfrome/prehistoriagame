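; Player controller for the co-op menu, handling hosting and joining of multiplayer games.
; On BeginPlay it shows the Coop_ENG widget and enables a locked cursor in Game and UI input.
; Hosting creates a two-connection, non-LAN session and opens Map_Demo_Prehistoria as a listen server.
; Joining runs an open console command with the given IP; both paths first play a connect sound, wait briefly, then switch to game-only input.
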(event Custom|hudMenu
  ;[1 1 1] hud menu
  (Utilities|IsValid (Variables|Default|GetCoop)
    (:Is%20Not%20Valid
      (bind _returnvalue (UserInterface|CreateWidget "/Game/Prog/Systemes/Menu/Widgets/ENG/Coop_ENG.Coop_ENG_C"))
      (bind _output_get (Variables|Default|SetCoop _returnvalue))
      (UserInterface|Viewport|AddtoViewport _output_get 0))))

(event Custom|initCursor
  ;[1 1 1] init cursor
  (Variables|Default|SetbShowMouseCursor true)
  (Input|SetInputModeGameandUI self 0 "LockAlways" true))

(event Custom|heberger
  (Audio|PlaySound2D "/Game/Sons/SFX/Menu/SFX_Connect.SFX_Connect" 1.0 1.0 0.0 0 0)
  (Utilities|FlowControl|Delay 1.0)
  (|Session self 2 false
    (:OnSuccess
      (Variables|Default|SetbShowMouseCursor false)
      (Input|SetInputModeGameOnly self)
      (Game|OpenLevel(byName) "Map_Demo_Prehistoria" true "listen"))))

(event Custom|rejoindre
  (params (ip :type String))
  (Audio|PlaySound2D "/Game/Sons/SFX/Menu/SFX_Connect.SFX_Connect" 1.0 1.0 0.0 0 0)
  (Utilities|FlowControl|Delay 1.0)
  (Development|PrintString ip)
  (Variables|Default|SetbShowMouseCursor false)
  (Development|ExecuteConsoleCommand (Utilities|String|Append "open " ip) 0)
  (Input|SetInputModeGameOnly self)
  (Development|PrintString "Hello"))

(event EventBeginPlay
  ;[1 1 1] init
  (CallFunction|HudMenu)
  (CallFunction|InitCursor))

(fn ConstructionScript)