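; Breakable foliage actor that swaps its static mesh for a destructible one when its health (Vie) runs out.
; PutMesh sets the visible mesh and deals one damage, while InitMeshBreak supplies the destructible asset used on break.
; After fracture, the debris clears, then the actor either destroys itself or restores mesh, collision and health after BP_GameMode's TempsRespawnRock delay, with a short fallback delay if the cast fails.
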(event OnComponentFracture(Destructible1)
  (params (HitPoint :type Vector%20%28by%20ref%29 :default "0, 0, 0") (HitDirection :type Vector%20%28by%20ref%29 :default "0, 0, 0"))
  (bind _normal_mesh (Variables|Default|Getnormal%20mesh))
  (Utilities|FlowControl|Delay 2.0)
  (Class|DestructibleComponent|SetDestructibleMesh (Variables|Default|GetDestructible1))
  (bind _asbp_game_mode (Utilities|Casting|CastToBP_GameMode (Game|GetGameMode))
    (:then
      (if (== (Variables|/Game/Prog/Systemes/Datas/BP_GameMode.BP_GameMode_C|GettempsRespawnRock _asbp_game_mode) -1.0)
        (Actor|DestroyActor)
        (else
          (Utilities|FlowControl|Delay (Variables|/Game/Prog/Systemes/Datas/BP_GameMode.BP_GameMode_C|GettempsRespawnRock _asbp_game_mode))
          (Rendering|SetVisibility _normal_mesh true false :!label _label)
          (Collision|SetCollisionEnabled _normal_mesh "QueryAndPhysics")
          (Variables|Default|Setvie (Variables|Default|GetvieMax))
          (Variables|Default|Setcasser? false))))
    (:CastFailed
      (Utilities|FlowControl|Delay 3.0)
      (goto _label))))

(event Custom|damage)

(event EventBeginPlay)

(event Collision|EventActorBeginOverlap
  (params (OtherActor :type Actor%20Object%20Reference)))

(event EventTick
  (params (DeltaSeconds :type Float%20%28single-precision%29)))

(fn ConstructionScript)

(fn PutMesh
  (params (mesh :type Static%20Mesh%20Object%20Reference))
  (Components|StaticMesh|SetStaticMesh (Variables|Default|Getnormal%20mesh) mesh)
  (CallFunction|MakeDamage 1))

(fn PutDestructMesh
  (bind _destructible1 (Variables|Default|GetDestructible1))
  (bind _destruct (Variables|Default|Getdestruct))
  (bind _normal_mesh (Variables|Default|Getnormal%20mesh))
  (if (not (Variables|Default|Getcasser?))
    (Utilities|IsValid _destruct
      (:Is%20Valid
        (Class|DestructibleComponent|SetDestructibleMesh _destructible1 _destruct)
        (Physics|SetSimulatePhysics _destructible1 true)
        (Class|KismetRenderingLibrary|SetCastInsetShadowforAllAttachments _destructible1 false false)
        (Rendering|SetVisibility _normal_mesh false false)
        (Collision|SetCollisionEnabled _normal_mesh "NoCollision")
        (Variables|Default|Setcasser? true))
      (:Is%20Not%20Valid
        (Development|PrintString "destruct none")))))

(fn MakeDamage
  (params (damage :type Integer))
  (Development|PrintString (Utilities|String|Append "vie : " (Utilities|String|ToString(Integer) (- (Variables|Default|Getvie) damage)) " >  0 = " (Utilities|String|ToString(Boolean) (> (- (Variables|Default|Getvie) damage) 0))))
  (if (> (- (Variables|Default|Getvie) damage) 0)
    (Variables|Default|Setvie (- (Variables|Default|Getvie) damage))
    (else
      (CallFunction|PutDestructMesh))))

(fn InitMeshBreak
  (params (destruct :type Destructible%20Mesh%20Object%20Reference))
  (Variables|Default|Setdestruct destruct))